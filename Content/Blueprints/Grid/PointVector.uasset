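; Grid point actor that holds velocity, density and U, with current and previous buffers, apparently as one cell of a fluid simulation.
; It starts with a random velocity, and Add functions accumulate velocity and density.
; Swap functions exchange current and previous values, together or per field, for double-buffered solving.
; Each tick it passes velocity to the WhiteFloaters effect and density to RedInk for visualisation.
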(event EventBeginPlay
  (Variables|Default|SetVelocity (* (Math|Random|RandomUnitVector) (Math|Random|RandomFloatinRange 1.0 1e+01))))

(event Collision|EventActorBeginOverlap
  (params (OtherActor :type Actor%20Object%20Reference)))

(event EventTick
  (params (DeltaSeconds :type Float%20%28single-precision%29))
  (Effects|Components|ParticleSystem|SetVectorParameter (Variables|Default|GetWhiteFloaters) "Velocity" (Variables|Default|GetVelocity))
  (Effects|Components|ParticleSystem|SetFloatParameter (Variables|Default|GetRedInk) "Density" (Variables|Default|GetDensity)))

(fn ConstructionScript)

(fn AddDensity
  (params (Amount :type Float%20%28double-precision%29))
  (Variables|Default|SetDensity (+ Amount (Variables|Default|GetDensity))))

(fn AddVelocity
  (params (Amount :type Vector))
  (Variables|Default|SetVelocity (+ Amount (Variables|Default|GetVelocity))))

(fn SwapVariables
  (Utilities|FlowControl|Sequence
    (:then_0
      (LocalVariables|SettempVel (Variables|Default|GetVelocity))
      (LocalVariables|SettempDensity (Variables|Default|GetDensity))
      (LocalVariables|SettempU (Variables|Default|GetU)))
    (:then_1
      (Variables|Default|SetVelocity (Variables|Default|GetPrevVelocity))
      (Variables|Default|SetDensity (Variables|Default|GetPrevDensity))
      (Variables|Default|SetU (Variables|Default|GetPrevU)))
    (:then_2
      (Variables|Default|SetPrevVelocity (LocalVariables|GettempVel))
      (Variables|Default|SetPrevDensity (LocalVariables|GettempDensity))
      (Variables|Default|SetPrevU (LocalVariables|GettempU)))))

(fn SwapDensities
  (Utilities|FlowControl|Sequence
    (:then_0
      (LocalVariables|SettempDensity (Variables|Default|GetDensity)))
    (:then_1
      (Variables|Default|SetDensity (Variables|Default|GetPrevDensity)))
    (:then_2
      (Variables|Default|SetPrevDensity (LocalVariables|GettempDensity)))))

(fn SwapVelocities
  (Utilities|FlowControl|Sequence
    (:then_0
      (LocalVariables|SettempVel (Variables|Default|GetVelocity)))
    (:then_1
      (Variables|Default|SetVelocity (Variables|Default|GetPrevVelocity)))
    (:then_2
      (Variables|Default|SetPrevVelocity (LocalVariables|GettempVel)))))

(fn SwapU
  (Utilities|FlowControl|Sequence
    (:then_0
      (LocalVariables|SettempU (Variables|Default|GetU)))
    (:then_1
      (Variables|Default|SetU (Variables|Default|GetPrevU)))
    (:then_2
      (Variables|Default|SetPrevU (LocalVariables|GettempU)))))